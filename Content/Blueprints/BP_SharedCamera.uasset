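; BP_SharedCamera is a shared view camera that frames the Bman game mode's tile grid.
; On BeginPlay it makes itself player controller 0's view target, then reads tile counts and tile size from BP_BmanGameMode.
; Math expressions centre it in X and Y, and its height equals the grid's X extent, a simplified placement that assumes a 90-degree FOV.
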(event EventBeginPlay
  ;[1 1 1] Simplified camera positioning for FOV == 90 deg
  (Game|Player|SetViewTargetwithBlend (Game|GetPlayerController 0) self 0.0 "VTBlend_Linear" 0.0 false)
  (bind _asbp_bman_game_mode (Utilities|Casting|CastToBP_BmanGameMode (Game|GetGameMode)))
  (Transformation|SetActorLocation (Math|Vector|MakeVector (|(((NumTiles*TileSize)/2)-(TileSize/2)) (Variables|/Script/Bman.BmanGameMode|GetNumTilesX _asbp_bman_game_mode) (Variables|/Script/Bman.BmanGameMode|GetTileSize _asbp_bman_game_mode)) (|(((NumTiles*TileSize)/2)-(TileSize/2)) (Variables|/Script/Bman.BmanGameMode|GetNumTilesY _asbp_bman_game_mode) (Variables|/Script/Bman.BmanGameMode|GetTileSize _asbp_bman_game_mode)) (* (Variables|/Script/Bman.BmanGameMode|GetNumTilesX _asbp_bman_game_mode) (Variables|/Script/Bman.BmanGameMode|GetTileSize _asbp_bman_game_mode))) false false))

(fn ConstructionScript)