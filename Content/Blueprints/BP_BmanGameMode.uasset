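; Game mode for a Bomberman-style match that ends a round and shows its result.
; EndRound pauses the game, then PresentResult creates the end screen and shows the mouse cursor.
; The outcome comes from DamagedPlayers: none or all damaged is a draw, otherwise player 0's pawn being damaged means Blue wins, else Red.
; The message goes to the end screen with both scores fixed at zero.
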(event `self.EndRound`
  (`GameplayStatics.SetGamePaused` true)
  (`self.PresentResult`))

(fn `PresentResult`
  (locals (Message :type Text) (Score0 :type Integer) (Score1 :type Integer))
  (bind _returnvalue (`KismetArrayLibrary.Array_Length` (`self.DamagedPlayers`)))
  (`|ExecutionSequence`
    (:`then_0`
      ;[1 1 1] Create and show end screen
      (bind _returnvalue_2 (`|CreateWidget` "/Game/UserInterface/BP_BmanEndScreen.BP_BmanEndScreen_C"))
      (`UserWidget.AddToViewport` _returnvalue_2 0)
      (set `PlayerController.bShowMouseCursor` true (`GameplayStatics.GetPlayerController` 0)))
    (:`then_1`
      ;[1 1 1] Check if result is a draw
      (bind _returnvalue_3 (`self.GetNumPlayers`))
      (if (or (== _returnvalue 0) (== _returnvalue _returnvalue_3))
        (set `local.Message` "Draw")
        (else
          ;[1 1 1] Find surving player
          (if (`KismetArrayLibrary.Array_Contains` (`self.DamagedPlayers`) (`Controller.K2_GetPawn` (`GameplayStatics.GetPlayerController` 0)))
            (set `local.Message` "Blue Won")
            (else
              (set `local.Message` "Red Won"))))))
    (:`then_2`
      ;[1 1 1] Set end screen info
      (`/Game/UserInterface/BP_BmanEndScreen.SetGameInfo` _returnvalue_2 (`local.Message`) 0 0))))

(fn `UserConstructionScript`)